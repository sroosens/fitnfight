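; BP_Door is a locked door that opens when a BP_Player holding at least one key overlaps its Box.
; It consumes a key, then a Timeline lerps the Cube vertically by MovingDistanceZ.
; Timeline event tracks switch the Niagara smoke on and off and trigger the player's camera shake.
; When the movement finishes, the actor destroys itself after a short delay.
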(event `self.Box.OnComponentBeginOverlap`
  (params (OverlappedComponent :type "PrimitiveComponent Object Reference") (OtherActor :type "Actor Object Reference") (OtherComp :type "PrimitiveComponent Object Reference") (OtherBodyIndex :type Integer) (bFromSweep :type Boolean) (SweepResult :type "HitResult Structure (by ref)"))
  (bind _niagara (`self.Niagara`))
  (bind _asbp_player (cast `/Game/_Main/Character/BP_Player` OtherActor))
  (if (> (`/Game/_Main/Character/BP_Player.NbKeys` _asbp_player) 0)
    (`/Engine/EditorBlueprintResources/StandardMacros.DecrementInt` (`/Game/_Main/Character/BP_Player.NbKeys` _asbp_player)
      (:`  `
        (bind (_direction _alpha) (`Timeline|Timeline` :!via `PlayFromStart`)
          (:`Update`
            (`SceneComponent.K2_SetRelativeLocation` (`self.Cube`) (`KismetMathLibrary.VLerp` (0.0 0.0 0.0) (`KismetMathLibrary.MakeVector` 0.0 0.0 (`self.MovingDistanceZ`)) _alpha) false false))
          (:`Finished`
            (`KismetSystemLibrary.Delay` 1.0)
            (`self.K2_DestroyActor`))
          (:`SmokeStart`
            (`ActorComponent.Activate` _niagara false))
          (:`SmokeEnd`
            (`ActorComponent.Deactivate` _niagara))
          (:`CamerShake`
            (bind _asbp_player_2 (cast `/Game/_Main/Character/BP_Player` (`GameplayStatics.GetPlayerCharacter` 0)))
            (`/Game/_Main/Character/BP_Player.UpdateCamerShake` _asbp_player_2)))))))

(fn `UserConstructionScript`)