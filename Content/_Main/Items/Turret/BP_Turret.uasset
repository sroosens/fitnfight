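; Turret that detects the player with PawnSensing, smoothly pitches toward them and repeatedly fires BP_Turret_Projectile while they are seen.
; Each tick it line-traces a fan of rays around the X axis and rebuilds a procedural mesh vision cone from the hits, so blocking geometry clips it.
; The cone is only a visual: firing depends on a seen flag that OnSeePawn sets and clears after roughly one sensing interval.
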(event `self.ReceiveBeginPlay`)

(event `self.ReceiveTick`
  (params (DeltaSeconds :type "Float (single-precision)"))
  (bind (_returnvalue_roll _returnvalue_pitch _returnvalue_yaw) (`KismetMathLibrary.BreakRotator` (`self.K2_GetActorRotation`)))
  (`self.UpdateDetectionConePosition`)
  (`self.GetHitDetectionCone`)
  (bind _asbp_player (cast `/Game/_Main/Character/BP_Player` (`GameplayStatics.GetPlayerCharacter` 0)))
  (if (`self.IsSeingPlayer`)
    (bind (_returnvalue_roll_2 _returnvalue_pitch_2) (`KismetMathLibrary.BreakRotator` (`KismetMathLibrary.FindLookAtRotation` (`self.K2_GetActorLocation`) (`self.K2_GetActorLocation` _asbp_player))))
    (`self.K2_SetActorRotation` (`KismetMathLibrary.RInterpTo` (`self.K2_GetActorRotation`) (`KismetMathLibrary.MakeRotator` _returnvalue_roll _returnvalue_pitch_2 _returnvalue_yaw) (`GameplayStatics.GetWorldDeltaSeconds`) 4.0))
    (`/Engine/EditorBlueprintResources/StandardMacros.DoOnce` false :!label _label
      (:`Completed`
        (`|ExecutionSequence`
          (:`then_0`
            (`|SpawnActorFromClass` "/Game/_Main/Items/Turret/BP_Turret_Projectile.BP_Turret_Projectile_C" (`KismetMathLibrary.MakeTransform` (`SceneComponent.K2_GetComponentLocation` (`self.ProjectileSpawn`)) (`self.K2_GetActorRotation`)) "Undefined" "OverrideRootScale" null null))
          (:`then_1`
            (`KismetSystemLibrary.Delay` 0.2)
            (goto _label :!via `Reset`)))))))

(event `self.PawnSensing.OnSeePawn`
  (params (Pawn :type "Pawn Object Reference"))
  (set `self.IsSeingPlayer` true)
  (`KismetSystemLibrary.Delay` (- (`PawnSensingComponent.SensingInterval` (`self.PawnSensing`)) (`self.GetActorTickInterval`)))
  (set `self.IsSeingPlayer` false))

(fn `GenerateDetectionCone`
  (locals (Index :type Integer) (`L Right Point` :type "Vector Structure") (`L Left Point` :type "Vector Structure"))
  (bind (_bblockinghit _binitialoverlap _time _distance _location _impactpoint _normal _impactnormal _physmat _hitactor _hitcomponent _hitbonename _bonename _hititem _elementindex _faceindex _tracestart _traceend) (`GameplayStatics.BreakHitResult` (`|GetArrayItem` (`self.Out Hits`) (`local.Index`))))
  (bind (_bblockinghit_2 _binitialoverlap_2 _time_2 _distance_2 _location_2 _impactpoint_2 _normal_2 _impactnormal_2 _physmat_2 _hitactor_2 _hitcomponent_2 _hitbonename_2 _bonename_2 _hititem_2 _elementindex_2 _faceindex_2 _tracestart_2 _traceend_2) (`GameplayStatics.BreakHitResult` (`|GetArrayItem` (`self.Out Hits`) (+ (`local.Index`) 1))))
  (for _index (range (`KismetArrayLibrary.Array_LastIndex` (`self.Out Hits`)))
    (set `local.Index` _index)
    (`|ExecutionSequence`
      (:`then_0`
        ;[1 1 1] Get Left & Right line trace points
        (if _bblockinghit
          (set `local.L Left Point` _location)
          (else
            (set `local.L Left Point` _traceend))))
      (:`then_1`
        (if _bblockinghit_2
          (set `local.L Right Point` _location_2)
          (else
            (set `local.L Right Point` _traceend_2))))
      (:`then_2`
        ;[1 1 1] Create a triangle from initial point with triangle sides from left and right lines
        (`ProceduralMeshComponent.CreateMeshSection_LinearColor` :`self` (`self.VisionCone`) :`SectionIndex` (`local.Index`) :`Vertices` (`|MakeArray` (- (`self.Start Point`) (`self.Start Point`)) (- (`local.L Left Point`) (`self.Start Point`)) (- (`local.L Right Point`) (`self.Start Point`))) :`Triangles` (`|MakeArray` 0 1 2))
        (`PrimitiveComponent.SetMaterial` (`self.VisionCone`) (`local.Index`) "/Game/_Main/Materials/MI_DetectionCone.MI_DetectionCone"))))
  (`SceneComponent.K2_SetRelativeRotation` (`self.VisionCone`) (* (`KismetMathLibrary.MakeRotFromX` (`SceneComponent.GetForwardVector` (`self.Turret`))) -1.0) false false))

(fn `GetHitDetectionCone`
  (locals (`Loc Current Angle` :type "Float (double-precision)"))
  (bind _start_point (`self.Start Point`))
  (for _index (range (+ (`self.Number Of Sections`) 1))
    ;[1 1 1] Trace line for each section and store hit
    (set `local.Loc Current Angle` (- (* _index (`self.D Angle`)) (`self.Half Cone Angle`)))
    (bind _outhit (`KismetSystemLibrary.LineTraceSingle` _start_point (+ _start_point (* (`KismetMathLibrary.RotateAngleAxis` (`self.GetActorForwardVector`) (`local.Loc Current Angle`) (1.0 0.0 0.0)) (`self.RangeCone`))) "TraceTypeQuery1"))
    (`KismetArrayLibrary.Array_Add` (`self.Out Hits`) _outhit))
  (`self.GenerateDetectionCone`))

(fn `InitDetectionCone`
  (`|ExecutionSequence`
    (:`then_0`
      (set `self.D Angle` (/ (* (`self.Half Cone Angle`) 2.0) (`self.Number Of Sections`))))
    (:`then_1`
      (set `self.Start Point` (+ (`KismetMathLibrary.MakeVector` 0.0) (`self.K2_GetActorLocation`))))
    (:`then_2`
      (`SceneComponent.K2_AddLocalOffset` (`self.VisionCone`) (`KismetMathLibrary.MakeVector` 0.0) false false))))

(fn `UpdateDetectionConePosition`
  (set `self.Start Point` (+ (`KismetMathLibrary.MakeVector` 0.0) (`self.K2_GetActorLocation`)))
  (`KismetArrayLibrary.Array_Clear` (`self.Out Hits`))
  (`ProceduralMeshComponent.ClearAllMeshSections` (`self.VisionCone`)))

(fn `UserConstructionScript`
  (`self.InitDetectionCone`)
  (`self.GetHitDetectionCone`))