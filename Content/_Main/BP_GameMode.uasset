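; BP_GameMode is the game mode Blueprint that runs a chronometer counting minutes, seconds and tenths of a second.
; While ChronoActive is true, Tick passes through a 0.1-second Delay to increment tenths, rolling overflow into seconds and minutes, so timing depends on frame rate.
; ResetChronometer zeroes the counters and starts counting, and StopChronometer clears the flag to halt it.
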(event `self.ReceiveBeginPlay`)

(event `self.ReceiveTick`
  (params (DeltaSeconds :type "Float (single-precision)"))
  ;[1 1 1] Chronometer
  (if (`self.ChronoActive`)
    (`KismetSystemLibrary.Delay` 0.1)
    (bind _output_get (set `self.TimeDSec` (+ (`self.TimeDSec`) 1)))
    (if (> _output_get 9)
      (set `self.TimeDSec` 0)
      (bind _output_get_2 (set `self.TimeSec` (+ (`self.TimeSec`) 1)))
      (if (> _output_get_2 59)
        (set `self.TimeMin` (+ (`self.TimeMin`) 1))
        (set `self.TimeSec` 0)))))

(event `ResetChronometer`
  (set `self.TimeDSec` 0)
  (set `self.TimeSec` 0)
  (set `self.TimeMin` 0)
  (set `self.ChronoActive` true))

(event `StopChronometer`
  (set `self.ChronoActive` false))

(fn `UserConstructionScript`)