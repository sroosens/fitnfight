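; Player character that moves on a single input axis, morphs between sphere and rectangle forms with different capsule heights, and reloads FirstLevel on R.
; Firing works only as a rectangle, spawning a projectile and shaving its Z scale each shot.
; An enlarged capsule trace detects walls while airborne.
; It drives a wall jump when input points away from the wall, and a per-tick gravity cut for wall sliding when not rising.
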(event `Key|R`
  (params (Key :type "Key Structure"))
  (:`Pressed`
    (`GameplayStatics.OpenLevel` "FirstLevel")))

(event `self.ReceiveTick`
  (params (DeltaSeconds :type "Float (single-precision)"))
  (`self.CheckSlowFall`))

(event `InputAxis|MoveForward`
  (params (AxisValue :type "Float (single-precision)"))
  (`self.AddMovementInput` (`KismetMathLibrary.GetForwardVector` (`self.GetControlRotation`)) AxisValue))

(event `InputAction|Jump`
  (params (Key :type "Key Structure"))
  (:`Pressed`
    (`self.Jump`)
    (`self.WallJump`))
  (:`Released`
    (`self.StopJumping`)))

(event `InputAction|Morph`
  (params (Key :type "Key Structure"))
  (:`Pressed`
    (`self.Morph`)))

(event `InputAction|Fire`
  (params (Key :type "Key Structure"))
  (bind _rectangle (`self.Rectangle`))
  (bind (_returnvalue_x _returnvalue_y _returnvalue_z) (`KismetMathLibrary.BreakVector` (`SceneComponent.K2_GetComponentScale` _rectangle)))
  (:`Pressed`
    (if (`self.IsRectangle`)
      (`|SpawnActorFromClass` "/Game/_Main/Blueprints/BP_Projectile.BP_Projectile_C" (`SceneComponent.K2_GetComponentToWorld` (`self.ProjectileArrow`)) "Undefined" "OverrideRootScale" null null)
      (`SceneComponent.SetWorldScale3D` _rectangle (`KismetMathLibrary.MakeVector` _returnvalue_x _returnvalue_y (- _returnvalue_z 0.02))))))

(fn `CheckSlowFall`
  (bind _returnvalue (`self.K2_GetActorLocation`))
  (bind _charactermovement (`self.CharacterMovement`))
  (bind _capsulecomponent (`self.CapsuleComponent`))
  (set `CharacterMovementComponent.GravityScale` 5.0 _charactermovement)
  (if (not (`NavMovementComponent.IsMovingOnGround` _charactermovement))
    (bind (_outhit _returnvalue_2) (`KismetSystemLibrary.CapsuleTraceSingle` _returnvalue _returnvalue (+ (`CapsuleComponent.CapsuleRadius` _capsulecomponent) 5.0) (`CapsuleComponent.CapsuleHalfHeight` _capsulecomponent) "TraceTypeQuery1"))
    (if _returnvalue_2
      (if (not (> (`.Z` (`KismetMathLibrary.BreakVector3f` (`SceneComponent.GetComponentVelocity` (`self.CapsuleComponent`)))) 0.0))
        (set `CharacterMovementComponent.GravityScale` 0.5 (`self.CharacterMovement`))))))

(fn `Morph`
  (bind _capsulecomponent (`self.CapsuleComponent`))
  (bind _sphere (`self.Sphere`))
  (bind _rectangle (`self.Rectangle`))
  (if (`self.IsRectangle`)
    (set `self.IsRectangle` false)
    (`SceneComponent.SetVisibility` _sphere true false)
    (`SceneComponent.SetVisibility` _rectangle false false)
    (`CapsuleComponent.SetCapsuleHalfHeight` _capsulecomponent 28.23 true)
    (else
      (set `self.IsRectangle` true)
      (`SceneComponent.SetVisibility` _sphere false false)
      (`SceneComponent.SetVisibility` _rectangle true false)
      (`CapsuleComponent.SetCapsuleHalfHeight` _capsulecomponent 47.7 true))))

(fn `UserConstructionScript`)

(fn `WallJump`
  (bind _returnvalue (`self.K2_GetActorLocation`))
  (bind _capsulecomponent (`self.CapsuleComponent`))
  (if (not (`NavMovementComponent.IsMovingOnGround` (`self.CharacterMovement`)))
    (bind (_outhit _returnvalue_2) (`KismetSystemLibrary.CapsuleTraceSingle` _returnvalue _returnvalue (+ (`CapsuleComponent.CapsuleRadius` _capsulecomponent) 5.0) (`CapsuleComponent.CapsuleHalfHeight` _capsulecomponent) "TraceTypeQuery1"))
    (if _returnvalue_2
      (`KismetSystemLibrary.PrintString` "WallJump")
      (bind _y (.y (`KismetMathLibrary.Normal` (`.ImpactNormal` (`GameplayStatics.BreakHitResult` _outhit)))))
      (if (> (* _y (`self.GetInputAxisValue`)) 0.0)
        (`self.LaunchCharacter` (`KismetMathLibrary.MakeVector` 0.0 (* _y (`self.LaunchStrength`)) 1500.0))))))