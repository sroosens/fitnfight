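; BP_Trap_Spike is a spike trap that kills a living BP_Player on overlapping its Box, passing TypeOfDeath to PlayerDead.
; Before the kill, it attaches a splatter decal to FBSpikeBack, using a dynamic material instance with a randomized Frame parameter.
; The decal's Y and Z follow the direction toward the player at SplashDistanceFromCenter, while X stays at a fixed offset from the trap.
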(event `self.Box.OnComponentBeginOverlap`
  (params (OverlappedComponent :type "PrimitiveComponent Object Reference") (OtherActor :type "Actor Object Reference") (OtherComp :type "PrimitiveComponent Object Reference") (OtherBodyIndex :type Integer) (bFromSweep :type Boolean) (SweepResult :type "HitResult Structure (by ref)"))
  (bind _returnvalue_x (`KismetMathLibrary.BreakVector` (`self.K2_GetActorLocation`)))
  (bind _returnvalue (`self.K2_GetActorLocation`))
  (bind _asbp_player (cast `/Game/_Main/Character/BP_Player` OtherActor))
  (if (not (`/Game/_Main/Character/BP_Player.IsDead` _asbp_player))
    ;[1 1 1] Create permanent splash decal onto trap
    (bind _returnvalue_2 (`KismetMaterialLibrary.CreateDynamicMaterialInstance` "/Game/_Main/Materials/MI_Splatter_Decal.MI_Splatter_Decal"))
    (`MaterialInstanceDynamic.SetScalarParameterValue` _returnvalue_2 "Frame" (`KismetMathLibrary.Conv_IntToDouble` (`KismetMathLibrary.RandomInteger` 11)))
    (bind (_returnvalue_x_2 _returnvalue_y _returnvalue_z) (`KismetMathLibrary.BreakVector` (+ (* (`KismetMathLibrary.Normal` (- (`self.K2_GetActorLocation` _asbp_player) _returnvalue)) (`self.SplashDistanceFromCenter`)) _returnvalue)))
    (`GameplayStatics.SpawnDecalAttached` _returnvalue_2 (20.0 45.0 20.0) (`self.FB_Spike_Back`) "None" (`KismetMathLibrary.MakeVector` (- _returnvalue_x 25.0) _returnvalue_y _returnvalue_z) (struct :`Yaw` -90.0) "KeepWorldPosition")
    (`/Game/_Main/Character/BP_Player.PlayerDead` _asbp_player (`self.Type Of Death`))))

(fn `UserConstructionScript`)