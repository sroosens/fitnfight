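; BP_Enemy is an enemy that kills the player when they overlap its Sphere1 component.
; An AI perception update plays a timeline, unless already running, that scales Sphere from its starting size and toggles whether the enemy is destroyable.
; The destroyable state also swaps the mesh material as a visual cue.
; When destroyed, it randomly may spawn a BP_Item_Projectile at its location.
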(event `self.ReceiveBeginPlay`
  (set `self.BaseScale` (`SceneComponent.K2_GetComponentScale` (`self.Sphere`))))

(event `self.Sphere1.OnComponentBeginOverlap`
  (params (OverlappedComponent :type "PrimitiveComponent Object Reference") (OtherActor :type "Actor Object Reference") (OtherComp :type "PrimitiveComponent Object Reference") (OtherBodyIndex :type Integer) (bFromSweep :type Boolean) (SweepResult :type "HitResult Structure (by ref)"))
  (bind _asbp_player (cast `/Game/_Main/Blueprints/BP_Player` OtherActor))
  (`/Game/_Main/Blueprints/BP_Player.PlayerDead` _asbp_player))

(event `self.AIPerception.OnPerceptionUpdated`
  (params (UpdatedActors :type "Array of Actor Object Reference (by ref)"))
  (if (not (`TimelineComponent.IsPlaying` (`self.ExpansionTimeline`)))
    (bind (_direction _expansion _destroyable) (`Timeline|ExpansionTimeline` :!via `PlayFromStart`)
      (:`Update`
        (`SceneComponent.SetWorldScale3D` (`self.Sphere`) (* _expansion (`self.BaseScale`)))
        (`self.UpdateDestroyable` _destroyable)))))

(event `self.ReceiveDestroyed`
  (if (`KismetMathLibrary.RandomBool`)
    (`|SpawnActorFromClass` "/Game/_Main/Blueprints/Items/BP_Item_Projectile.BP_Item_Projectile_C" (`KismetMathLibrary.MakeTransform` (`self.K2_GetActorLocation`)) "Undefined" "OverrideRootScale" null null)))

(fn `UpdateDestroyable`
  (params (Value :type "Float (double-precision)"))
  (bind _output_get (set `self.IsDestroyable` (> Value 0.0)))
  (if _output_get
    (`PrimitiveComponent.SetMaterial` (`self.StaticMesh`) 0 "/Game/StarterContent/Materials/M_Tech_Hex_Tile_Pulse.M_Tech_Hex_Tile_Pulse")
    (else
      (`PrimitiveComponent.SetMaterial` (`self.StaticMesh`) 0 "/Game/StarterContent/Props/Materials/M_TableRound.M_TableRound")))
  (return))

(fn `UserConstructionScript`)