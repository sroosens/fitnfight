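; BP_WinGate is a level goal trigger that ends play with a win screen when the player reaches it.
; Its Box overlap responds only to BP_Player, pausing the game and stopping the current level sound held by BP_GameMode.
; It then creates and shows the W_Win widget, switches input to Game and UI, and shows the mouse cursor.
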(event `self.Box.OnComponentBeginOverlap`
  (params (OverlappedComponent :type "PrimitiveComponent Object Reference") (OtherActor :type "Actor Object Reference") (OtherComp :type "PrimitiveComponent Object Reference") (OtherBodyIndex :type Integer) (bFromSweep :type Boolean) (SweepResult :type "HitResult Structure (by ref)"))
  (bind _returnvalue (`GameplayStatics.GetPlayerController` 0))
  (cast `/Game/_Main/Character/BP_Player` OtherActor)
  (`GameplayStatics.SetGamePaused` true)
  ;[1 1 1] Stop current sound playing
  (bind _asbp_game_mode (cast `/Game/_Main/BP_GameMode` (`GameplayStatics.GetGameMode`)))
  (`AudioComponent.Stop` (`/Game/_Main/BP_GameMode.CurLevelSound` _asbp_game_mode))
  ;[1 1 1] Display Win Widget
  (bind _returnvalue_2 (`|CreateWidget` "/Game/_Main/Widgets/W_Win.W_Win_C"))
  (`UserWidget.AddToViewport` _returnvalue_2 0)
  (`WidgetBlueprintLibrary.SetInputMode_GameAndUIEx` _returnvalue null)
  (set `PlayerController.bShowMouseCursor` true _returnvalue))

(fn `UserConstructionScript`)