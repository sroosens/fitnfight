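; Player character for a Paper2D side-view platformer, with run, jump, wall jump, wall slide and timeline-driven dash.
; Tick picks flipbooks and facing, detects wall slides by capsule trace and updates walk VFX.
; Any damage or the R key kills, leaving a splatter decal, then respawns at the last checkpoint or PlayerStart.
; Also handles HUD, pause menu, key and size-up pickups, Niagara effects, camera shake and gamepad rumble.
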(event `Key|R`
  (params (Key :type "Key Structure"))
  (:`Pressed`
    (`self.PlayerDead`)))

(event `self.ReceiveBeginPlay`
  (bind _returnvalue (`|CreateWidget` "/Game/_Main/Widgets/W_HUD.W_HUD_C" (`GameplayStatics.GetPlayerController` 0)))
  (`UserWidget.AddToViewport` _returnvalue 0))

(event `InputAction|Morph`
  (params (Key :type "Key Structure")))

(event `self.ReceiveTick`
  (params (DeltaSeconds :type "Float (single-precision)"))
  ;[0 0.3636 1] Even Tick
  (`|ExecutionSequence`
    (:`then_0`
      (`self.UpdateAnimation`))
    (:`then_1`
      (`self.CheckSliding`))
    (:`then_2`
      (`self.UpdateWalkVFX`))))

(event `Key|AnyKey`
  (params (Key :type "Key Structure"))
  ;[1 1 1] Check if Gamepad is currently used
  (:`Pressed`
    (if (`KismetInputLibrary.Key_IsGamepadKey` Key)
      (set `self.GamePadUsed` true)
      (else
        (set `self.GamePadUsed` false)))))

(event `InputAxis|MoveRightLeft`
  (params (AxisValue :type "Float (single-precision)"))
  ;[1 1 1] Manage Movement
  (if (not (`self.IsDead`))
    (`self.AddMovementInput` (`KismetMathLibrary.GetForwardVector` (`self.GetControlRotation`)) AxisValue)))

(event `InputAction|Escape` :paused true
  (params (Key :type "Key Structure"))
  (bind _returnvalue (`GameplayStatics.GetPlayerController` 0))
  ;[1 1 1] Manage Pause Menu
  (:`Pressed`
    (if (not (`GameplayStatics.IsGamePaused`))
      (bind _returnvalue_2 (`|CreateWidget` "/Game/_Main/Widgets/W_PauseMenu.W_PauseMenu_C"))
      (`UserWidget.AddToViewport` _returnvalue_2 0)
      (`GameplayStatics.SetGamePaused` true)
      (`WidgetBlueprintLibrary.SetInputMode_GameAndUIEx` _returnvalue null)
      (set `PlayerController.bShowMouseCursor` true _returnvalue)
      (else
        (`Widget.RemoveFromParent` _returnvalue_2)
        (`GameplayStatics.SetGamePaused` false)))))

(event `InputAction|Jump`
  (params (Key :type "Key Structure"))
  ;[1 1 1] Manage Jump
  (:`Pressed`
    (if (not (`self.IsDead`))
      (`self.Jump`)
      (set `self.IsSliding` false)
      (`self.CheckWallJump`)
      (`self.UpdateJumpVFX`)))
  (:`Released`
    (`self.StopJumping`)))

(event `CheckWallJump`
  (bind _returnvalue (`self.K2_GetActorLocation`))
  (bind _capsulecomponent (`self.CapsuleComponent`))
  ;[1 1 1] Wall Jump
  (if (not (`NavMovementComponent.IsMovingOnGround` (`self.CharacterMovement`)))
    (bind (_outhit _returnvalue_2) (`KismetSystemLibrary.CapsuleTraceSingle` _returnvalue _returnvalue (+ (`CapsuleComponent.CapsuleRadius` _capsulecomponent) 2.5) (`CapsuleComponent.CapsuleHalfHeight` _capsulecomponent) "TraceTypeQuery1"))
    (if _returnvalue_2
      (bind _y (.y (`KismetMathLibrary.Normal` (`.ImpactNormal` (`GameplayStatics.BreakHitResult` _outhit)))))
      (if (> (* _y (`self.GetInputAxisValue`)) 0.0)
        _
        (else
          _))
      (`self.LaunchCharacter` (`KismetMathLibrary.MakeVector` 0.0 (* _y (`self.JumpStrength`)) 1500.0)))))

(event `CheckSliding`
  (bind _returnvalue (`self.K2_GetActorLocation`))
  (bind _charactermovement (`self.CharacterMovement`))
  (bind _capsulecomponent (`self.CapsuleComponent`))
  (bind _charactermovement_2 (`self.CharacterMovement`))
  (bind _capsulecomponent_2 (`self.CapsuleComponent`))
  (bind (_velocity_x _velocity_y _velocity_z) (`KismetMathLibrary.BreakVector` (`MovementComponent.Velocity` _charactermovement_2)))
  ;[1 1 1] Slide
  (`FXSystemComponent.SetFloatParameter` (`self.NS_WallSlide`) "Velocity" 0.0)
  (set `CharacterMovementComponent.GravityScale` 5.0 _charactermovement)
  (if (`NavMovementComponent.IsMovingOnGround` _charactermovement)
    (set `self.IsSliding` false)
    (else
      (bind (_outhit _returnvalue_2) (`KismetSystemLibrary.CapsuleTraceSingle` _returnvalue _returnvalue (+ (`CapsuleComponent.CapsuleRadius` _capsulecomponent) 2.0) (`CapsuleComponent.CapsuleHalfHeight` _capsulecomponent) "TraceTypeQuery1"))
      (if _returnvalue_2
        (if (> (`.Z` (`KismetMathLibrary.BreakVector3f` (`SceneComponent.GetComponentVelocity` _capsulecomponent_2))) 0.0)
          (set `self.IsSliding` false)
          (else
            (set `self.IsSliding` true)
            (set `CharacterMovementComponent.GravityScale` (`self.Wall Sliding Scale`) _charactermovement_2)
            (set `MovementComponent.Velocity` (`KismetMathLibrary.MakeVector` _velocity_x _velocity_y (`KismetMathLibrary.FClamp` _velocity_z (`self.Wall Sliding Velocity`) 2000.0)) _charactermovement_2)
            (`self.UpdateSlideVFX` (>= (`KismetMathLibrary.DegAsin` (`KismetMathLibrary.Dot_VectorVector` (`.Normal` (`GameplayStatics.BreakHitResult` _outhit)) (`SceneComponent.GetRightVector` _capsulecomponent_2))) 0.0))))))))

(event `InputAction|Dash`
  (params (Key :type "Key Structure"))
  ;[1 1 1] Manage Dash
  (:`Pressed`
    (if (not (`self.IsDead`))
      (if (not (`self.IsDashing`))
        (set `self.IsDashing` true)
        (bind (_direction _distancemultiplier) (`Timeline|Movement` :!via `PlayFromStart`)
          (:`Update`
            (bind _directionvector (`self.GetCurrentDirVector`))
            (set `MovementComponent.Velocity` (* _directionvector (* _distancemultiplier (`self.Dash Distance Scale`))) (`self.CharacterMovement`))
            (`self.UpdateDashVFX`)
            (set `self.IsDashing` false)))))))

(event `PlayerDead`
  (bind _paperflipbook (`self.PaperFlipbook`))
  ;[1 1 1] Manage Death
  (if (not (`self.IsDead`))
    (`self.VFX Die`)
    (set `self.IsDead` true)
    (`GameplayStatics.PlaySound2D` "/Game/_Main/Sounds/hurt_c_08-102842_01.hurt_c_08-102842_01" 1.0 1.0 0.0 null null)
    (`ActorComponent.Deactivate` (`self.NS_Walk`))
    (`ActorComponent.Deactivate` (`self.NS_WallSlide`))
    (`ActorComponent.Deactivate` (`self.CharacterMovement`))
    (`PaperFlipbookComponent.SetLooping` _paperflipbook false)
    (`PaperFlipbookComponent.SetFlipbook` _paperflipbook "/Game/_Main/Character/Animation/Die/FB_DieSuit.FB_DieSuit")
    (`self.UpdateCamerShake`)
    (`KismetSystemLibrary.Delay` 2.5)
    (`self.Respawn`)))

(event `AddItem`
  (params (Type :type "/Game/_Main/Items/Enum_Items Enum" :default "NewEnumerator0"))
  ;[1 1 1] Manage Collected Items
  (switch `/Game/_Main/Items/Enum_Items` Type
    (:`NewEnumerator0`
      (`self.CharacterSizeUp`))
    (:`NewEnumerator1`
      (`/Engine/EditorBlueprintResources/StandardMacros.IncrementInt` (`self.NbKeys`)))))

(event `self.CapsuleComponent.OnComponentBeginOverlap`
  (params (OverlappedComponent :type "PrimitiveComponent Object Reference") (OtherActor :type "Actor Object Reference") (OtherComp :type "PrimitiveComponent Object Reference") (OtherBodyIndex :type Integer) (bFromSweep :type Boolean) (SweepResult :type "HitResult Structure (by ref)"))
  ;[1 1 1] Manage CheckPoint
  (if (`self.ActorHasTag` OtherActor "Checkpoint")
    (`KismetSystemLibrary.PrintString` "Nw checkpoint!")
    (set `self.CurrentCheckpoint` OtherActor)
    (bind _outactors (`GameplayStatics.GetAllActorsOfClass` "/Game/_Main/Items/BP_CheckPoint.BP_CheckPoint_C"))
    (for _array_element _outactors
      (if (== _array_element (`self.CurrentCheckpoint`))
        (`/Game/_Main/Items/BP_CheckPoint.Activate` _array_element)
        (else
          (`/Game/_Main/Items/BP_CheckPoint.Deactivate` _array_element))))))

(event `Respawn`
  (bind _paperflipbook (`self.PaperFlipbook`))
  ;[1 1 1] Manage Respawn
  (`SceneComponent.SetVisibility` (`self.PaperFlipbook`) false false)
  (`/Engine/EditorBlueprintResources/StandardMacros.IsValid` (`self.CurrentCheckpoint`)
    (:`Is Valid`
      (bind _outactors (`GameplayStatics.GetAllActorsOfClass` "/Game/_Main/Items/BP_CheckPoint.BP_CheckPoint_C"))
      (for _array_element _outactors
        (if (== _array_element (`self.CurrentCheckpoint`))
          (break)))
      (`self.K2_SetActorLocation` (+ (`SceneComponent.K2_GetComponentLocation` (`/Game/_Main/Items/BP_CheckPoint.TPPoint` _array_element)) (0.0 0.0 40.0)) false true))
    (:`Is Not Valid`
      (`KismetSystemLibrary.PrintString` "Checkpoint invalid!")
      (bind _returnvalue (`GameplayStatics.GetActorOfClass` "/Script/Engine.PlayerStart"))
      (bind _returnvalue_location (`KismetMathLibrary.BreakTransform` (`self.GetTransform` _returnvalue)))
      (`self.K2_SetActorLocation` _returnvalue_location false true)))
  (`self.Stop VFX Die`)
  (`self.UpdateRespawnVFX`)
  (`ActorComponent.Activate` (`self.CharacterMovement`) false)
  (`PaperFlipbookComponent.SetLooping` _paperflipbook true)
  (`PaperFlipbookComponent.Play` _paperflipbook)
  (`KismetSystemLibrary.Delay` 1.0)
  (`SceneComponent.SetVisibility` (`self.PaperFlipbook`) true false)
  (`ActorComponent.Activate` (`self.NS_WallSlide`) false)
  (`ActorComponent.Activate` (`self.NS_Walk`) false)
  (set `self.IsDead` false))

(event `self.ReceiveAnyDamage`
  (params (Damage :type "Float (single-precision)") (DamageType :type "DamageType Object Reference") (InstigatedBy :type "Controller Object Reference") (DamageCauser :type "Actor Object Reference"))
  ;[1 1 1] Damage Dealer
  (`self.PlayerDead`))

(event `UpdateAnimation`
  (bind _paperflipbook (`self.PaperFlipbook`))
  ;[0.217 1 0.5686] Animation Character
  (if (not (`self.IsDead`))
    (bind _currentfb (`self.GetCurrentAnimation`))
    (`PaperFlipbookComponent.SetFlipbook` _paperflipbook _currentfb)
    (`PaperFlipbookComponent.Play` _paperflipbook)
    (`self.UpdateAnimationSide`)))

(event `UpdateCamerShake`
  ;[1 0.7608 0.3176] VFX Camera Shake
  (`PlayerCameraManager.StartCameraShake` :`self` (`GameplayStatics.GetPlayerCameraManager` 0) :`ShakeClass` "/Game/_Main/Character/CameraShake/BP_CameraShake.BP_CameraShake_C" :`Scale` 0.08)
  (if (`self.GamepadUsed`)
    (`PlayerController.PlayDynamicForceFeedback` (`GameplayStatics.GetPlayerController` 0) 0.05 0.1 true true true true)))

(event `UpdateDashVFX`
  ;[1 0.7608 0.3176] VFX Dash
  (if (>= (`self.GetInputAxisValue`) 0.0)
    ;;[1 1 1] VFX Direction
    (`FXSystemComponent.SetFloatParameter` (`self.NS_DashLines`) "SpeedScale" 1.0)
    (else
      (`FXSystemComponent.SetFloatParameter` (`self.NS_DashLines`) "SpeedScale" -1.0)))
  (`ActorComponent.Activate` (`self.NS_DashLines`) false)
  (`PlayerCameraManager.StartCameraShake` :`self` (`GameplayStatics.GetPlayerCameraManager` 0) :`ShakeClass` "/Game/_Main/Character/CameraShake/BP_CameraShake.BP_CameraShake_C" :`Scale` 0.03)
  (if (`self.GamepadUsed`)
    (`PlayerController.PlayDynamicForceFeedback` (`GameplayStatics.GetPlayerController` 0) 0.05 0.1 true true true true)))

(event `UpdateJumpVFX`
  (bind _ns_jump (`self.NS_Jump`))
  ;[1 0.7591 0.3184] VFX Jump
  (if (`NavMovementComponent.IsFalling` (`self.CharacterMovement`))
    _
    (else
      _))
  (`ActorComponent.Activate` _ns_jump false)
  (`GameplayStatics.PlaySound2D` "/Game/_Main/Sounds/8-bit-jump.8-bit-jump" 1.0 1.0 0.0 null null)
  (`KismetSystemLibrary.Delay` 0.05)
  (`ActorComponent.Deactivate` _ns_jump))

(event `UpdateWalkVFX`
  ;[1 0.7591 0.3184] VFX Walk
  (if (`NavMovementComponent.IsMovingOnGround` (`self.CharacterMovement`))
    (`FXSystemComponent.SetFloatParameter` (`self.NS_Walk`) "Velocity" (`KismetMathLibrary.FClamp` (`KismetMathLibrary.Abs` (`KismetMathLibrary.VSize` (`self.GetVelocity`)))))
    (else
      (`FXSystemComponent.SetFloatParameter` (`self.NS_Walk`) "Velocity" 0.0))))

(event `UpdateSlideVFX`
  (params (SlidingRight :type Boolean))
  (bind _ns_wallslide (`self.NS_WallSlide`))
  ;[1 0.7608 0.3176] VFX Slide
  (if SlidingRight
    (set `self.SlidingRight` false)
    (`FXSystemComponent.SetVectorParameter` _ns_wallslide "PositionOffset" (-25.0 0.0 0.0))
    (else
      (set `self.SlidingRight` true)
      (`FXSystemComponent.SetVectorParameter` _ns_wallslide "PositionOffset" (25.0 0.0 0.0))))
  (`FXSystemComponent.SetFloatParameter` _ns_wallslide "Velocity" 1.0)
  (`PlayerCameraManager.StartCameraShake` :`self` (`GameplayStatics.GetPlayerCameraManager` 0) :`ShakeClass` "/Game/_Main/Character/CameraShake/BP_CameraShake_Slide.BP_CameraShake_Slide_C" :`Scale` 0.06)
  (if (`self.GamepadUsed`)
    (`PlayerController.PlayDynamicForceFeedback` (`GameplayStatics.GetPlayerController` 0) 0.02 0.1 true true true true)))

(event `UpdateRespawnVFX`
  ;[1 0.7608 0.3176] VFX Respawn
  (`ActorComponent.Activate` (`self.NS_Soul`) false))

(event `VFX Die`
  (bind (_returnvalue_x _returnvalue_y _returnvalue_z) (`KismetMathLibrary.BreakVector` (`self.K2_GetActorLocation`)))
  ;[1 0.7608 0.3176] VFX Die
  (`ActorComponent.Activate` (`self.NS_Blood`) false)
  (bind _returnvalue (`KismetMaterialLibrary.CreateDynamicMaterialInstance` "/Game/_Main/Materials/MI_Splatter_Decal.MI_Splatter_Decal"))
  (`MaterialInstanceDynamic.SetScalarParameterValue` _returnvalue "Frame" (`KismetMathLibrary.Conv_IntToDouble` (`KismetMathLibrary.RandomInteger` 11)))
  (`GameplayStatics.SpawnDecalAtLocation` _returnvalue (30.0 70.0 70.0) (`KismetMathLibrary.MakeVector` (- _returnvalue_x 120.0) _returnvalue_y (- _returnvalue_z (`CapsuleComponent.CapsuleHalfHeight` (`self.CapsuleComponent`)))) (struct)))

(event `Stop VFX Die`
  (bind (_direction _alpha) (`Timeline|HitTimeline` :!via `Stop`)
    (:`Update`
      (`MeshComponent.SetScalarParameterValueOnMaterials` (`self.PaperFlipbook`) "HitActive" _alpha))))

(fn `CharacterSizeDown`
  (bind _capsulecomponent (`self.CapsuleComponent`))
  (bind _returnvalue (/ (`SceneComponent.K2_GetComponentScale` _capsulecomponent) 1.2))
  (if (< (`KismetMathLibrary.VSize` _returnvalue) 0.2)
    (`self.PlayerDead`)
    (else
      (`SceneComponent.SetWorldScale3D` _capsulecomponent _returnvalue))))

(fn `CharacterSizeUp`
  (bind _capsulecomponent (`self.CapsuleComponent`))
  (`SceneComponent.SetWorldScale3D` _capsulecomponent (* (`SceneComponent.K2_GetComponentScale` _capsulecomponent) 1.2)))

(fn `GetCurrentAnimation`
  (returns (CurrentFB :type "PaperFlipbook Object Reference"))
  (`PaperFlipbookComponent.SetLooping` (`self.PaperFlipbook`) true)
  (if (`self.IsSliding`)
    (`PaperFlipbookComponent.SetLooping` (`self.PaperFlipbook`) false)
    (return "/Game/_Main/Character/Animation/Slide/FB_SlideSuit.FB_SlideSuit")
    (elif (not (`NavMovementComponent.IsMovingOnGround` (`self.CharacterMovement`)))
      (`PaperFlipbookComponent.SetLooping` (`self.PaperFlipbook`) false)
      (return "/Game/_Main/Character/Animation/Jump/FB_JumpSuit.FB_JumpSuit")
      (elif (> (`KismetMathLibrary.VSize` (`MovementComponent.Velocity` (`self.CharacterMovement`))) 0.0)
        (return "/Game/_Main/Character/Animation/Run/FB_RunSuit_3.FB_RunSuit_3")
        (else
          (return "/Game/_Main/Character/Animation/Idle/FB_SuitIdle_2.FB_SuitIdle_2"))))))

(fn `GetCurrentDirVector`
  (returns (DirectionVector :type "Vector Structure"))
  (if (>= (`self.GetInputAxisValue`) 0.0)
    (return (`self.GetActorForwardVector`))
    (else
      (return (* (`self.GetActorForwardVector`) -1.0)))))

(fn `UpdateAnimationSide`
  (bind (_returnvalue_x _returnvalue_y) (`KismetMathLibrary.BreakVector` (`self.GetVelocity`)))
  (if (`self.IsSliding`)
    (if (`self.SlidingRight`)
      ;[1 1 1] Sliding Side
      (`SceneComponent.SetRelativeScale3D` (`self.PaperFlipbook`) (2.5 2.5 2.5))
      (else
        (`SceneComponent.SetRelativeScale3D` (`self.PaperFlipbook`) (-2.5 2.5 2.5))))
    (elif (>= _returnvalue_y 0.0)
      ;[1 1 1] Running Side
      (`SceneComponent.SetRelativeScale3D` (`self.PaperFlipbook`) (2.5 2.5 2.5))
      (else
        (`SceneComponent.SetRelativeScale3D` (`self.PaperFlipbook`) (-2.5 2.5 2.5))))))

(fn `UserConstructionScript`)