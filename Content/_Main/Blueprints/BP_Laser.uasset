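; BP_Laser is a laser hazard that switches on and off on a looping timer and damages BP_Player on contact.
; While enabled, Tick grows the beam toward its max distance along the chosen Left/Right/Up/Down world axis and line traces along it.
; A hit shortens the beam, positions the impact Niagara effect and applies damage to the player.
; The construction script also sets the Niagara color and width and runs one beam update.
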(event `self.ReceiveBeginPlay`
  (bind _niagaralaser (`self.NiagaraLaser`))
  (`FXSystemComponent.SetColorParameter` _niagaralaser "Color" (struct :`R` 0.776042 :`G` 0.013 :`A` 1.0))
  (`FXSystemComponent.SetColorParameter` (`self.NiagaraLaserImpact`) "Color" (struct :`R` 0.776042 :`G` 0.013 :`A` 1.0))
  (`FXSystemComponent.SetFloatParameter` _niagaralaser "Width" (`self.Width`))
  (`KismetSystemLibrary.K2_SetTimerDelegate` (delegate `LaserProcess`) 3.0 true))

(event `LaserProcess`
  (if (`self.Enabled`)
    (`self.DisableLaser`)
    (else
      (`self.EnableLaser`))))

(event `self.ReceiveTick`
  (params (DeltaSeconds :type "Float (single-precision)"))
  (`self.UpdateBeam` DeltaSeconds))

(event `EnableLaser`
  (bind _niagaralaser (`self.NiagaraLaser`))
  ;[1 1 1] Enable Laser Beam
  (set `self.Enabled` true)
  (`SceneComponent.SetVisibility` _niagaralaser true false)
  (`ActorComponent.Activate` _niagaralaser true))

(event `DisableLaser`
  (bind _niagaralaser (`self.NiagaraLaser`))
  ;[1 1 1] Disable Laser Beam
  (set `self.Enabled` false)
  (`SceneComponent.SetVisibility` _niagaralaser false false)
  (`SceneComponent.SetVisibility` (`self.NiagaraLaserImpact`) false false)
  (set `self.CurrentDistance` 0.0)
  (`FXSystemComponent.SetVectorParameter` (`self.NiagaraLaser`) "LaserEnd" (`self.K2_GetActorLocation`))
  (`ActorComponent.Deactivate` _niagaralaser))

(event `UpdateBeam`
  (params (`Delta Seconds` :type "Float (double-precision)"))
  (bind _returnvalue (`self.K2_GetActorLocation`))
  (if (`self.Enabled`)
    (`|ExecutionSequence`
      (:`then_0`
        (bind _direction (`self.GetCapsuleVectorDirection`))
        (bind _returnvalue_2 (+ _returnvalue (* _direction (`self.CurrentDistance`))))
        (set `self.TraceEnd` _returnvalue_2)
        (bind (_outhit _returnvalue_3) (`KismetSystemLibrary.LineTraceSingle` _returnvalue _returnvalue_2 "TraceTypeQuery1"))
        (set `self.Hit` _returnvalue_3)
        (bind (_bblockinghit _binitialoverlap _time _distance _location _impactpoint _normal _impactnormal _physmat _hitactor) (`GameplayStatics.BreakHitResult` _outhit))
        (set `self.HitLocation` _location)
        (`FXSystemComponent.SetVectorParameter` (`self.NiagaraLaser`) "LaserEnd" (select `bool` (`self.Hit`) :`false` (`self.TraceEnd`) :`true` (`self.HitLocation`)))
        (`SceneComponent.SetVisibility` (`self.NiagaraLaserImpact`) (`self.Hit`) false)
        (`SceneComponent.K2_SetWorldLocation` (`self.NiagaraLaserImpact`) (`self.HitLocation`) false false)
        (if (`self.Hit`)
          (set `self.CurrentDistance` (`KismetMathLibrary.VSize` (- (`self.HitLocation`) (`self.K2_GetActorLocation`))))
          ;[1 1 1] Check if Player is Hit
          (bind _asbp_player (cast `/Game/_Main/Blueprints/BP_Player` _hitactor))
          (`GameplayStatics.ApplyDamage` _asbp_player 100.0)))
      (:`then_1`
        (`self.UpdateSpeed` `Delta Seconds`)))))

(event `UpdateSpeed`
  (params (`Delta Seconds` :type "Float (double-precision)"))
  (bind _currentdistance (`self.CurrentDistance`))
  (if (< _currentdistance (`self.MaxDistance`))
    (set `self.CurrentDistance` (+ _currentdistance (* `Delta Seconds` (`self.ProgagationSpeed`))))))

(fn `GetCapsuleVectorDirection`
  (returns (Direction :type "Vector Structure"))
  (switch `/Game/_Main/Blueprints/Effects/Laser/Enum_Laser_Direction` (`self.Direction`)
    (:`NewEnumerator0`
      (return (0.0 -1.0 0.0)))
    (:`NewEnumerator1`
      (return (0.0 1.0 0.0)))
    (:`NewEnumerator2`
      (return (0.0 0.0 1.0)))
    (:`NewEnumerator3`
      (return (0.0 0.0 -1.0)))))

(fn `UserConstructionScript`
  (bind _niagaralaser (`self.NiagaraLaser`))
  (`FXSystemComponent.SetColorParameter` _niagaralaser "Color" (struct :`R` 0.776042 :`G` 0.013 :`A` 1.0))
  (`FXSystemComponent.SetColorParameter` (`self.NiagaraLaserImpact`) "Color" (struct :`R` 0.776042 :`G` 0.013 :`A` 1.0))
  (`FXSystemComponent.SetFloatParameter` _niagaralaser "Width" (`self.Width`))
  (`self.UpdateBeam` 1.0))