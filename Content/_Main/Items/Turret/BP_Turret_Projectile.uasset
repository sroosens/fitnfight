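; BP_Turret_Projectile is the turret's projectile, which kills the player on contact.
; Each Tick it runs a small stationary box trace at its location on the Visibility channel, skipping an ignore list added to at BeginPlay.
; Any hit destroys the projectile, and a hit on BP_Player also calls PlayerDead.
; A timed self-destruct exists but is unconnected, so it never runs.
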(event `self.ReceiveBeginPlay`
  (`KismetArrayLibrary.Array_Add` (`self.Actors to Ignore`)))

(event `self.ReceiveTick`
  (params (DeltaSeconds :type "Float (single-precision)"))
  (bind _returnvalue (`self.K2_GetActorLocation`))
  (bind (_outhit _returnvalue_2) (`KismetSystemLibrary.BoxTraceSingle` _returnvalue _returnvalue (5.0 5.0 5.0) (struct) "TraceTypeQuery1" false (`self.Actors to Ignore`) "None" true (struct :`R` 1.0 :`A` 1.0) (struct :`G` 1.0 :`A` 1.0) 0.1))
  (if _returnvalue_2
    (`self.K2_DestroyActor`)
    (bind _asbp_player (cast `/Game/_Main/Character/BP_Player` (`.HitActor` (`GameplayStatics.BreakHitResult` _outhit))))
    (`/Game/_Main/Character/BP_Player.PlayerDead` _asbp_player)))

(fn `UserConstructionScript`)